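; BP_MainGameMode is the SphereJam game mode that tracks the target score, flags the win and starts the level audio.
; AddTargetPoint subtracts the given points from TargetScore, so the score counts down.
; Tick polls TargetScore and sets GameWin only when it equals exactly zero.
; BeginPlay plays the Audio component, then applies the volume multiplier stored in the BP_instance game instance.
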(event Custom|AddTargetPoint
  (params (AddScorePoint :type Integer))
  (Variables|Default|SetTargetScore (- (Variables|Default|GetTargetScore) AddScorePoint)))

(event EventTick
  (params (DeltaSeconds :type Float%20%28single-precision%29))
  (if (== (Variables|Default|GetTargetScore) 0)
    (Variables|Default|SetGameWin true)))

(event EventBeginPlay
  (bind _audio (Variables|Default|GetAudio))
  ;[1 1 1] Audio
  (Audio|Components|Audio|Play _audio 0.0)
  (bind _asbp_instance (Utilities|Casting|CastToBP_instance (Game|GetGameInstance)))
  (Audio|Components|Audio|SetVolumeMultiplier _audio (Variables|/Game/SphereJam/Core/GameModes/BP_instance.BP_instance_C|GetVolumeMultiple _asbp_instance) :!class /Script/Engine.AudioComponent))

(fn ConstructionScript)