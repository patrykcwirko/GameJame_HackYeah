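; Sphere character Blueprint, apparently an older version by its name, with melee combat, weapon attachment and health.
; Left click cycles a three-step montage combo behind an IsAttacking gate, which this graph never clears.
; Melee box overlaps deal fixed damage to other Player-tagged actors, and received damage reduces Health.
; At zero Health it plays a non-looping animation and disables capsule collision, while EquipWeapon snaps a weapon to the skeletal mesh.
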(event OnComponentBeginOverlap(MeleeBoxColision)
  (params (OverlappedComponent :type Primitive%20Component%20Object%20Reference) (OtherActor :type Actor%20Object%20Reference) (OtherComp :type Primitive%20Component%20Object%20Reference) (OtherBodyIndex :type Integer) (bFromSweep :type Boolean) (SweepResult :type Hit%20Result%20Structure%20%28by%20ref%29))
  ;[1 0.122 0.1917] Combat System
  (if (Actor|ActorHasTag OtherActor "Player")
    (if (!= OtherActor self)
      (Game|Damage|ApplyDamage OtherActor 22.0 0 self "/Script/Engine.DamageType"))))

(event EventEquipWeapon
  (params (Weapon :type BP%20Weapon%20Base%20Object%20Reference))
  ;[0.6458 0.2917 1] Equip Weapon
  (Transformation|AttachComponentToComponent Weapon (Variables|Default|GetSkeletalMesh) "None" "SnapToTarget" "SnapToTarget" "SnapToTarget" true))

(event Game|Damage|EventAnyDamage
  (params (Damage :type Float%20%28single-precision%29) (DamageType :type Damage%20Type%20Object%20Reference) (InstigatedBy :type Controller%20Object%20Reference) (DamageCauser :type Actor%20Object%20Reference))
  (bind _skeletalmesh (Variables|Default|GetSkeletalMesh))
  ;[1 0.122 0.1917] Combat System
  (Variables|Default|SetHealth (- (Variables|Default|GetHealth) Damage))
  (if (<= (Variables|Default|GetHealth) 0.0)
    (Components|Animation|SetAnimationMode _skeletalmesh "AnimationBlueprint")
    (Components|Animation|PlayAnimation _skeletalmesh 0 false)
    (Collision|SetCollisionEnabled (Variables|Default|GetCapsuleColision) "NoCollision")))

(event Input|MouseEvents|LeftMouseButton
  (params (Key :type Key%20Structure :default "None"))
  (bind _skeletalmesh (Variables|Default|GetSkeletalMesh))
  ;[0.1499 1 0.2353] Input
  (:Pressed
    (Variables|Default|SetMelee%20Speed 1.2)
    ;[0.1232 0.8094 1] Combat animation play
    (if (not (Variables|Default|GetisAttacking))
      (Variables|Default|SetisAttacking true)
      (switch int (Variables|Default|GetAttack%20Count)
        (:0
          (Variables|Default|SetAttack%20Count 1)
          (Animation|Montage|PlayMontage _skeletalmesh 0 (Variables|Default|GetMelee%20Speed)))
        (:1
          (Variables|Default|SetAttack%20Count 2)
          (Animation|Montage|PlayMontage _skeletalmesh 0 (Variables|Default|GetMelee%20Speed)))
        (:2
          (Variables|Default|SetAttack%20Count 0)
          (Animation|Montage|PlayMontage _skeletalmesh 0 (Variables|Default|GetMelee%20Speed)))))))

(fn ConstructionScript)